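; Player controller for a multiplayer game, managing each player's lobby and in-game UI, chat, character selection, score and kicks.
; GM switches between lobby widget and GameUI, also routing incoming chat to the active one.
; MyGameMode relays messages to all controllers and refreshes the scoreboard when kills or deaths change; MyGameInstance supplies the LAN name and loading screen.
; Enter opens game chat, Tab shows the scoreboard, and G/H manually add kills/deaths.
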(event Custom|AddLobbyWB
  (params (ServerName :type String) (ServerMap :type String) (ServerMode :type String) (ServerSlots :type Integer))
  ;[1 1 1] Create Lobby Widget
  (Variables|Default|SetbShowMouseCursor true)
  (bind _returnvalue (UserInterface|CreateWidget "/Game/Ui/LobbyWB.LobbyWB_C" 0 (Utilities|Text|ToText(String) ServerName) (Utilities|Text|ToText(String) ServerMap) (Utilities|Text|ToText(String) ServerMode) ServerSlots))
  (bind _output_get (Variables|Default|SetLobbyWB _returnvalue))
  (UserInterface|Viewport|AddtoViewport _output_get 1))

(event Custom|AddPlayer
  (params (Player :type Text) (PlayerIndex :type Integer) (CharacterImage :type Object%20Object%20Reference))
  ;[1 1 1] Add player to list
  (Default|AddPlayertoList (Variables|Default|GetLobbyWB) Player PlayerIndex CharacterImage))

(event Custom|SetGameMode
  (params (GameMode :type Integer))
  (Variables|Default|SetGameMode GameMode))

(event Custom|PlayerDataSetupOnServer
  (params (Lan_Name :type String))
  (bind _output_get (Variables|Default|SetLan_Name Lan_Name))
  (Class|AdvancedSessionsLibrary|SetPlayerName self (select (Class|AdvancedSessionsLibrary|HasOnlineSubsystem "STEAM") (Class|AdvancedSessionsLibrary|GetPlayerName self) _output_get))
  (CallFunction|SetUpFinished))

(event Custom|CreateGameUi
  (bind _returnvalue (UserInterface|CreateWidget "/Game/Ui/Game/GameUI.GameUI_C"))
  (bind _output_get (Variables|Default|SetGameUI _returnvalue))
  (UserInterface|Viewport|AddtoViewport _output_get 0)
  (Input|SetInputModeGameOnly self)
  (Variables|Default|SetbShowMouseCursor false))

(event Custom|Add%20Death
  (Math|Integer|IncrementInt (Variables|Default|GetDeath)
    (:%20%20
      (Variables|Default|SetKD (/ (Math|Conversions|ToFloat(Integer) (Variables|Default|GetKills)) (Math|Conversions|ToFloat(Integer) (Variables|Default|GetDeath))))
      (bind _asmy_game_mode (Utilities|Casting|CastToMyGameMode (Game|GetGameMode)))
      (Default|UpdateScoreBoard _asmy_game_mode))))

(event Custom|ClearScoreBoard
  (Default|Clear (Variables|/Game/Ui/Game/GameUI.GameUI_C|GetScoreBoard (Variables|Default|GetGameUI))))

(event Custom|TeleportOnOwningClient
  (params (NewLocation :type Vector))
  (Default|TeleportPlayeronServer (Variables|Default|GetMain%20Character) NewLocation))

(event Custom|AddPlayerScoreBoard
  (params (Name :type String) (Kills :type Integer) (Deaths :type Integer) (position :type Integer) (KD :type Float%20%28single-precision%29) (IsOwnPlayer? :type Boolean) (In%20Notin%20TOp%20List :type Boolean))
  (Default|AddPlayer (Variables|/Game/Ui/Game/GameUI.GameUI_C|GetScoreBoard (Variables|Default|GetGameUI)) Name Kills Deaths position KD IsOwnPlayer? In%20Notin%20TOp%20List))

(event Custom|SetUpNewGameModeAndUI
  (params (GM :type Integer) (LoadingScreenTime :type Float%20%28single-precision%29))
  (bind _lobbywb (Variables|Default|GetLobbyWB))
  (bind _output_get (Variables|Default|SetGM GM))
  (if (!= _output_get 0)
    (Utilities|FlowControl|Delay LoadingScreenTime)
    (Widget|SetVisibility (Variables|Default|GetLobbyWB) "Collapsed")
    (Utilities|FlowControl|Delay 0.2)
    (bind _asmy_game_mode (Utilities|Casting|CastToMyGameMode (Game|GetGameMode)))
    (Default|CreateGameUIonEachPlayer _asmy_game_mode)
    (else
      (Widget|RemovefromParent (Variables|Default|GetGameUI))
      (Utilities|FlowControl|Delay 0.2)
      (Widget|SetVisibility _lobbywb "Visible")
      (Input|SetInputModeUIOnly self _lobbywb "DoNotLock")
      (Variables|Default|SetbShowMouseCursor true))))

(event Custom|Add%20Kill
  (Math|Integer|IncrementInt (Variables|Default|GetKills)
    (:%20%20
      (if (== (Variables|Default|GetDeath) 0)
        (Variables|Default|SetKD (Math|Conversions|ToFloat(Integer) (Variables|Default|GetKills)))
        (else
          (Variables|Default|SetKD (/ (Math|Conversions|ToFloat(Integer) (Variables|Default|GetKills)) (Math|Conversions|ToFloat(Integer) (Variables|Default|GetDeath))))))
      (bind _asmy_game_mode (Utilities|Casting|CastToMyGameMode (Game|GetGameMode)))
      (Default|UpdateScoreBoard _asmy_game_mode))))

(event Custom|SendImportantServerMessage
  (params (Message :type Text) (Delay :type Float%20%28single-precision%29) (Color :type Linear%20Color%20Structure) (Size :type Integer))
  (bind _gameui (Variables|Default|GetGameUI))
  (bind _importantservermessagebox (Variables|/Game/Ui/Game/GameUI.GameUI_C|GetImportantServerMessageBox _gameui))
  (bind _box (Variables|/Game/Ui/Game/ImportantServerMessageBox.ImportantServerMessageBox_C|GetBox _importantservermessagebox))
  (bind _returnvalue (UserInterface|CreateWidget "/Game/Ui/Game/ImportantServerMessage.ImportantServerMessage_C" 0 Message Delay Color Size))
  (Widget|Panel|AddChild _box _returnvalue)
  (Utilities|FlowControl|Delay Delay)
  (Class|PanelWidget|RemoveChild _box _returnvalue))

(event Custom|AddMessageFromServerToEachPlayer
  (params (Message :type String) (Color :type Slate%20Color%20Structure) (IsServerMessage :type Boolean))
  (bind _self self)
  (bind _playername (Class|AdvancedSessionsLibrary|GetPlayerName _self))
  (bind _chatmessagestructure (Utilities|Struct|MakeChatMessageStructure _playername Message Color IsServerMessage))
  (bind _asmy_game_mode (Utilities|Casting|CastToMyGameMode (Game|GetGameMode)))
  (for _array_element (Variables|/Game/Blueprints/MyGameMode.MyGameMode_C|GetAllPCs _asmy_game_mode)
    (bind _asmy_player_controller (Utilities|Casting|CastToMyPlayerController _array_element))
    (CallFunction|AddMessagetoChat _asmy_player_controller _chatmessagestructure))
  (bind _asmy_game_mode_2 (Utilities|Casting|CastToMyGameMode (Game|GetGameMode)))
  (Default|AddMessagetoChatHistory _asmy_game_mode_2 _chatmessagestructure))

(event Custom|SetServerData
  (params (ServerName :type String) (ServerMode :type String))
  (Default|SetServerData (Variables|/Game/Ui/Game/GameUI.GameUI_C|GetScoreBoard (Variables|Default|GetGameUI)) ServerName ServerMode))

(event Custom|StartCountdownCenter
  (params (Minutes :type Integer) (Seconds :type Integer) (Disable%20Movement? :type Boolean))
  (Default|StartCountdown (Variables|/Game/Ui/Game/GameUI.GameUI_C|GetCountDownCenter (Variables|Default|GetGameUI)) Minutes Seconds)
  (if Disable%20Movement?
    (bind _asmain_character (Utilities|Casting|CastToMainCharacter (Game|GetPlayerCharacter 0)))
    (Variables|/Game/ThirdPersonBP/Blueprints/MainCharacter.MainCharacter_C|SetWaiting%20for%20Start _asmain_character true)
    (Utilities|FlowControl|Delay (Math|Conversions|ToFloat(Integer) (+ (* Minutes 60) Seconds)))
    (Variables|/Game/ThirdPersonBP/Blueprints/MainCharacter.MainCharacter_C|SetWaiting%20for%20Start _asmain_character false)))

(event Custom|StartInGameTimer
  (params (Minutes :type Integer) (Seconds :type Integer) (CountUp? :type Boolean))
  (Default|StartCountdown (Variables|/Game/Ui/Game/GameUI.GameUI_C|GetCountDownRight (Variables|Default|GetGameUI)) Minutes Seconds CountUp?))

(event Custom|SelectCharacterMulti
  (params (Same? :type Boolean) (SelectedCharacterNumber :type Integer) (SelectedCharacterClass :type Pawn%20Class%20Reference))
  (if Same?
    (Variables|Default|SetSelectedCharacterNumber 0)
    (Variables|Default|SetSelectedCharacterClass 0)
    (else
      (Variables|Default|SetSelectedCharacterNumber SelectedCharacterNumber)
      (Variables|Default|SetSelectedCharacterClass SelectedCharacterClass))))

(event Custom|ClearPlayerList
  ;[1 1 1] Clear player list
  (Default|ClearPlayerList (Variables|Default|GetLobbyWB)))

(event Custom|UpdateServerFromPC
  (bind _asmy_game_mode (Utilities|Casting|CastToMyGameMode (Game|GetGameMode)))
  (Default|UpdateServer _asmy_game_mode))

(event Custom|UpdateAvaliableCharactersNoTeam
  (params (NewParam :type Array%20of%20Booleans))
  (for (_array_element _array_index) NewParam
    (bind _ascharacter_button (Utilities|Casting|CastToCharacterButton (Class|PanelWidget|GetChildat (Variables|/Game/Ui/LobbyWB.LobbyWB_C|GetCharacterBox1 (Variables|Default|GetLobbyWB)) _array_index)))
    (Default|ToggleEnable _ascharacter_button _array_element)))

(event Custom|SelectCharacterOnServer
  (params (Same? :type Boolean) (Selection :type Integer) (SelectCharacterClass :type Pawn%20Class%20Reference))
  (CallFunction|SelectCharacterMulti Same? Selection SelectCharacterClass))

(event Custom|SetTeamForLobbyWB
  (params (Team :type Integer) (Same? :type Boolean)))

(event Custom|JoinOrLeaveTeam
  (params (Team :type Integer) (Same? :type Boolean)))

(event Custom|LoadingScreen
  ;[1 1 1] Loading Screen
  (Widget|RemovefromParent (Variables|Default|GetLobbyWB))
  (bind _asmy_game_instance (Utilities|Casting|CastToMyGameInstance (Game|GetGameInstance)))
  (Default|ShowLoadingScreen _asmy_game_instance))

(event Custom|AddMessageToChat
  (params (NewParam :type Chat%20Message%20Structure%20Structure))
  (if (== (Variables|Default|GetGM) 0)
    (Default|AddChildtoChat (Variables|/Game/Ui/LobbyWB.LobbyWB_C|GetChatBox (Variables|Default|GetLobbyWB)) NewParam)
    (else
      (Default|AddChildtoChat (Variables|/Game/Ui/Game/GameUI.GameUI_C|GetGameChatWindow (Variables|Default|GetGameUI)) NewParam self))))

(event Custom|Kick
  (params (KickIndex :type Integer))
  (switch int KickIndex
    (:0
      (Game|OpenLevel(byName) "Kicked")
      (|DestroySession self))
    (:1
      (Game|OpenLevel(byName) "ServerFull")
      (|DestroySession self))))

(event Custom|HideChat
  (Variables|Default|SetIsChatOpen? false)
  (Input|SetInputModeGameOnly self)
  (Variables|Default|SetbShowMouseCursor false)
  (for _array_element (Variables|Default|GetGameChatArray)
    (Default|ChatOpened _array_element false)))

(event Custom|SetUpFinished
  ;[1 1 1] HZ nakoy
  (bind _asmy_game_mode (Utilities|Casting|CastToMyGameMode (Game|GetGameMode)))
  (Default|Continue _asmy_game_mode))

(event Custom|HideLoadingScreen
  (bind _asmy_game_instance (Utilities|Casting|CastToMyGameInstance (Game|GetGameInstance)))
  (Default|HideLoadingScreen _asmy_game_instance))

(event Custom|UpdateNumberOfPlayers
  (params (currentPlayers :type Integer))
  ;[1 1 1] Update Player-Number
  (Variables|/Game/Ui/LobbyWB.LobbyWB_C|SetcurrentPlayers (Variables|Default|GetLobbyWB) currentPlayers))

(event Custom|PlayerDataSetup
  (bind _asmy_game_instance (Utilities|Casting|CastToMyGameInstance (Game|GetGameInstance)))
  (bind _output_get (Variables|Default|SetLan_Name (Variables|/Game/Blueprints/MyGameInstance.MyGameInstance_C|GetLan_Name _asmy_game_instance)))
  (CallFunction|PlayerDataSetuponServer _output_get))

(event Custom|Add%20GameChatChildToArray
  (params (NewItem :type Game%20Chat%20Message%20Child%20Object%20Reference%20%28by%20ref%29))
  (Utilities|Array|Add (Variables|Default|GetGameChatArray) NewItem))

(event EventBeginPlay
  (bind _asmain_character (Utilities|Casting|CastToMainCharacter (Game|GetPlayerCharacter 0)))
  (Variables|Default|SetMain%20Character _asmain_character))

(event Input|KeyboardEvents|Enter
  (params (Key :type Key%20Structure :default "None"))
  (bind _gameui (Variables|Default|GetGameUI))
  (bind _gamechatwindow (Variables|/Game/Ui/Game/GameUI.GameUI_C|GetGameChatWindow _gameui))
  (:Pressed
    (if (not (== (Variables|Default|GetGM) 0))
      (if (not (Variables|Default|GetIsChatOpen?))
        (Variables|Default|SetIsChatOpen? true)
        (Input|SetInputModeUIOnly self 0 "DoNotLock")
        (Variables|Default|SetbShowMouseCursor true)
        (Widget|SetKeyboardFocus (Variables|/Game/Ui/Game/GameChatWindow.GameChatWindow_C|GetEditableSerchBox _gamechatwindow))
        (for _array_element (Variables|Default|GetGameChatArray)
          (Default|ChatOpened _array_element true))
        (Class|ScrollBox|ScrolltoEnd (Variables|/Game/Ui/Game/GameChatWindow.GameChatWindow_C|GetScrollBox_Chat _gamechatwindow))))))

(event Input|KeyboardEvents|H
  (params (Key :type Key%20Structure :default "None"))
  (:Pressed
    (CallFunction|AddDeath)))

(event Input|KeyboardEvents|G
  (params (Key :type Key%20Structure :default "None"))
  (:Pressed
    (CallFunction|AddKill)))

(event Input|KeyboardEvents|Tab
  (params (Key :type Key%20Structure :default "None"))
  (bind _gameui (Variables|Default|GetGameUI))
  (bind _scoreboard (Variables|/Game/Ui/Game/GameUI.GameUI_C|GetScoreBoard _gameui))
  (:Pressed
    (Widget|SetVisibility _scoreboard "HitTestInvisible"))
  (:Released
    (Widget|SetVisibility _scoreboard "Collapsed")))

(fn ConstructionScript)