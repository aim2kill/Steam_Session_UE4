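; Player controller for the multiplayer lobby, bridging the lobby game mode and each player's lobby and loading-screen widgets.
; Events create the lobby widget, maintain its player list and count, and handle kicks by returning to the menu and destroying the session.
; Chat messages are relayed through the game mode to every controller and saved to history.
; Name setup uses the Steam name or a LAN name from the game instance, then updates the server.
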(event Custom|AddLobbyWB
  (params (ServerName :type String) (ServerMap :type String) (ServerMode :type String) (ServerSlots :type Integer))
  ;[1 1 1] Create Lobby Widget
  (Variables|Default|SetbShowMouseCursor true)
  (bind _returnvalue (UserInterface|CreateWidget "/Game/Ui/LobbyWB.LobbyWB_C" 0 (Utilities|Text|ToText(String) ServerName) (Utilities|Text|ToText(String) ServerMap) (Utilities|Text|ToText(String) ServerMode) ServerSlots))
  (bind _output_get (Variables|Default|SetLobbyWB _returnvalue))
  (UserInterface|Viewport|AddtoViewport _output_get 1))

(event Custom|AddPlayer
  (params (Player :type Text) (PlayerIndex :type Integer))
  ;[1 1 1] Add player to list
  (Default|AddPlayertoList (Variables|Default|GetLobbyWB) Player PlayerIndex))

(event Custom|LoadingScreen
  ;[1 1 1] Loading Screen
  (Widget|RemovefromParent (Variables|Default|GetLobbyWB))
  (bind _returnvalue (UserInterface|CreateWidget "/Game/Ui/LoadingScreen.LoadingScreen_C" self))
  (UserInterface|Viewport|AddtoViewport _returnvalue 0))

(event Custom|PlayerDataSetupOnServer
  (params (Lan_Name :type String))
  (bind _output_get (Variables|Default|SetLan_Name Lan_Name))
  (Class|AdvancedSessionsLibrary|SetPlayerName self (select (Class|AdvancedSessionsLibrary|HasOnlineSubsystem "STEAM") (Class|AdvancedSessionsLibrary|GetPlayerName self) _output_get))
  (bind _aslobby_game_mode (Utilities|Casting|CastToLobbyGameMode (Game|GetGameMode)))
  (Default|UpdateServer _aslobby_game_mode))

(event Custom|AddMessageFromServerToEachPlayer
  (params (Message :type String) (Color :type Slate%20Color%20Structure) (IsServerMessage :type Boolean))
  (bind _self self)
  (bind _playername (Class|AdvancedSessionsLibrary|GetPlayerName _self))
  (bind _chatmessagestructure (Utilities|Struct|MakeChatMessageStructure _playername Message Color IsServerMessage))
  (bind _aslobby_game_mode (Utilities|Casting|CastToLobbyGameMode (Game|GetGameMode)))
  (for _array_element (Variables|/Game/Blueprints/LobbyGameMode.LobbyGameMode_C|GetAllPCs _aslobby_game_mode)
    (bind _aslobby_player_controller (Utilities|Casting|CastToLobbyPlayerController _array_element))
    (CallFunction|AddMessagetoChat _aslobby_player_controller _chatmessagestructure))
  (bind _aslobby_game_mode_2 (Utilities|Casting|CastToLobbyGameMode (Game|GetGameMode)))
  (Default|AddMessagetoChatHistory _aslobby_game_mode_2 _chatmessagestructure))

(event Custom|ClearPlayerList
  ;[1 1 1] Clear player list
  (Default|ClearPlayerList (Variables|Default|GetLobbyWB)))

(event Custom|AddMessageToChat
  (params (NewParam :type Chat%20Message%20Structure%20Structure))
  (Default|AddChildtoChat (Variables|/Game/Ui/LobbyWB.LobbyWB_C|GetChatBox (Variables|Default|GetLobbyWB)) NewParam))

(event Custom|Kick
  ;[1 1 1] kick player
  (Game|OpenLevel(byName) "Menu")
  (|DestroySession self))

(event Custom|SetUpFinished
  (bind _aslobby_game_mode (Utilities|Casting|CastToLobbyGameMode (Game|GetGameMode)))
  (Default|Continue _aslobby_game_mode))

(event Custom|UpdateNumberOfPlayers
  (params (currentPlayers :type Integer))
  ;[1 1 1] Update Player-Number
  (Variables|/Game/Ui/LobbyWB.LobbyWB_C|SetcurrentPlayers (Variables|Default|GetLobbyWB) currentPlayers))

(event Custom|PlayerDataSetup
  (bind _asmy_game_instance (Utilities|Casting|CastToMyGameInstance (Game|GetGameInstance)))
  (bind _output_get (Variables|Default|SetLan_Name (Variables|/Game/Blueprints/MyGameInstance.MyGameInstance_C|GetLan_Name _asmy_game_instance)))
  (CallFunction|PlayerDataSetuponServer _output_get))

(fn ConstructionScript)