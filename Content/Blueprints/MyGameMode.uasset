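; Multiplayer game mode that runs the server lobby and match flow, from login and map travel to returning players to the lobby.
; It tracks controllers, pushing player lists, server messages and chat history, and kicking overflow players.
; Matches spawn characters at shuffled mode-specific points and start countdowns and timers by mode.
; The scoreboard ranks players by repeatedly extracting the highest KD, showing each client the top list plus their own row.
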(event Custom|JoinGame
  (bind _returnvalue (Game|GetPlayerController 0))
  ;[1 1 1] Start Game - servertravel
  (if (Utilities|Enum|Equal(Enum) (Variables|Default|GetServerMap) "Map1")
    ;;[0.8817 1 0] Add Custom Map
    (Development|ExecuteConsoleCommand "servertravel/Game/Maps/Map1" _returnvalue :!label _label)
    (elif (Utilities|Enum|Equal(Enum) (Variables|Default|GetServerMap) "Map2")
      (Development|ExecuteConsoleCommand "servertravel/Game/Maps/Map2" _returnvalue)
      (else
        (goto _label))))
  (bind _asmy_game_instance (Utilities|Casting|CastToMyGameInstance (Game|GetGameInstance)))
  (Default|JoinGame _asmy_game_instance))

(event Custom|AddMessageToChatHistory
  (params (Data :type Chat%20Message%20Structure%20Structure))
  (Utilities|Array|Add (Variables|Default|GetMessageLOG) Data))

(event Custom|UpdateServer
  (bind _allpcs (Variables|Default|GetAllPCs))
  (bind _returnvalue (Utilities|Array|Length _allpcs))
  (if (> _returnvalue (Variables|Default|GetServerSlots))
    (CallFunction|KickPlayer (- _returnvalue 1) 1)
    ;[1 1 1] Update Server
    (Utilities|FlowControl|Delay 0.2))
  ;;[1 1 1] clear list from each player
  (for _array_element (Variables|Default|GetAllPCs)
    (bind _asmy_player_controller (Utilities|Casting|CastToMyPlayerController _array_element))
    (Default|ClearPlayerList _asmy_player_controller)
    ;;[1 1 1] Add each player to the list
    (for (_array_element_2 _array_index) (Variables|Default|GetAllPCs)
      (Default|AddPlayer _asmy_player_controller (Utilities|Text|ToText(String) (Class|AdvancedSessionsLibrary|GetPlayerName _array_element_2)) _array_index)))
  ;;[1 1 1] Update number of players
  (for _array_element_3 (Variables|Default|GetAllPCs)
    (bind _asmy_player_controller_2 (Utilities|Casting|CastToMyPlayerController _array_element_3))
    (Default|UpdateNumberOfPlayers _asmy_player_controller_2 (Utilities|Array|Length (Variables|Default|GetAllPCs)))))

(event Custom|SendImportantServerMessage
  (params (Message :type Text) (Delay :type Float%20%28single-precision%29) (Color :type Linear%20Color%20Structure :default "(R=1.000000,G=1.000000,B=1.000000,A=1.000000)") (Size :type Integer))
  (for _array_element (Variables|Default|GetAllPCs)
    (bind _asmy_player_controller (Utilities|Casting|CastToMyPlayerController _array_element))
    (Default|SendImportantServerMessage _asmy_player_controller Message Delay Color Size)))

(event Custom|StartGamePlay
  (if (Utilities|Enum|Equal(Enum) (Variables|Default|GetServerMode) "Death Mutch")
    (for _array_element (Variables|Default|GetAllPCs)
      (bind _asmy_player_controller (Utilities|Casting|CastToMyPlayerController _array_element))
      (Default|StartinGameTimer _asmy_player_controller 2 30 false))
    (elif (Utilities|Enum|Equal(Enum) (Variables|Default|GetServerMode) "1 vs 1")
      (for _array_element_2 (Variables|Default|GetAllPCs)
        (bind _asmy_player_controller_2 (Utilities|Casting|CastToMyPlayerController _array_element_2))
        (Default|StartinGameTimer _asmy_player_controller_2 0 5 true))
      (elif (Utilities|Enum|Equal(Enum) (Variables|Default|GetServerMode) "No CharSelect")
        (for _array_element_3 (Variables|Default|GetAllPCs)
          (bind _asmy_player_controller_3 (Utilities|Casting|CastToMyPlayerController _array_element_3))
          (Default|StartinGameTimer _asmy_player_controller_3 1 0 false))))))

(event Custom|MovePlayersToLobby
  (bind _outactors (Actor|GetAllActorsOfClass "/Game/ThirdPersonBP/Blueprints/MainCharacter.MainCharacter_C"))
  (for _array_element _outactors
    (Actor|DestroyActor _array_element))
  (CallFunction|ToggleinGame false)
  (for _array_element_2 (Variables|Default|GetAllPCs)
    (bind _asmy_player_controller (Utilities|Casting|CastToMyPlayerController _array_element_2))
    (Default|SetUpNewGameModeandUI _asmy_player_controller 0 0.0)
    (Variables|Default|SetPlyersInGamePlay (Variables|Default|GetAllPCs))
    (Variables|/Game/Blueprints/MyPlayerController.MyPlayerController_C|SetKills _asmy_player_controller 0)
    (Variables|/Game/Blueprints/MyPlayerController.MyPlayerController_C|SetDeath _asmy_player_controller 0)))

(event Custom|SendServerMssage
  (params (Message :type String))
  (bind _asmy_player_controller (Utilities|Casting|CastToMyPlayerController (Game|GetPlayerController 0)))
  (Default|AddMessagefromServertoEachPlayer _asmy_player_controller Message (Utilities|Struct|MakeSlateColor "(R=1.000000,G=1.000000,B=0.000000,A=1.000000)") true))

(event Custom|Continue
  ;[1 1 1] Add each Player Controller to list and add server information
  ;;[1 1 1] HZ nakoy
  (CallFunction|SendServerMssage (Utilities|String|Append (Class|AdvancedSessionsLibrary|GetPlayerName (stale EventPostLogin NewPlayer)) " : " "Joined"))
  (Default|AddLobbyWB (stale EventPostLogin _asmy_player_controller) (Variables|Default|GetServerName) (Variables|Default|GetServerMap) (Variables|Default|GetServerMode) (Variables|Default|GetServerSlots))
  (CallFunction|UpdateServer)
  (for _array_element (Variables|Default|GetMessageLOG)
    (bind _asmy_player_controller (Utilities|Casting|CastToMyPlayerController (stale EventPostLogin NewPlayer)))
    (Default|AddMessagetoChat _asmy_player_controller _array_element)))

(event Custom|KickPlayer
  (params (Index :type Integer) (KickIndex :type Integer))
  ;[1 1 1] Kick Player
  (bind _asmy_player_controller (Utilities|Casting|CastToMyPlayerController (Utilities|Array|Get(acopy) (Variables|Default|GetAllPCs) Index)))
  (Default|Kick _asmy_player_controller KickIndex)
  ;[1 1 1] Start Game - servertravel
  (CallFunction|SendServerMssage (Utilities|String|Append (Class|AdvancedSessionsLibrary|GetPlayerName _asmy_player_controller) " : " "Kicked")))

(event Custom|SetGameMode
  (params (GameMode :type Integer))
  (Variables|Default|SetGameMode GameMode))

(event Custom|SetServerDataGameplay
  (bind _asmy_game_instance (Utilities|Casting|CastToMyGameInstance (Game|GetGameInstance)))
  (Variables|Default|SetServerName (Variables|/Game/Blueprints/MyGameInstance.MyGameInstance_C|GetServerName _asmy_game_instance))
  (Variables|Default|SetServerMode (Variables|/Game/Blueprints/MyGameInstance.MyGameInstance_C|GetServerMode _asmy_game_instance)))

(event Custom|UpdateScoreBoard
  (bind _kds (Variables|Default|GetKDs))
  (bind _indexofmaxvalue (Math|Float|MaxOfFloatArray _kds))
  (Utilities|Array|Clear (Variables|Default|GetPlayerAddedToScoreBoard))
  (Utilities|Array|Clear (Variables|Default|GetCopies))
  (Utilities|Array|Clear (Variables|Default|GetKDs))
  (bind _output_get (Variables|Default|SetCopies (Variables|Default|GetPlyersInGamePlay)))
  (for _array_element _output_get
    (bind _asmy_player_controller (Utilities|Casting|CastToMyPlayerController _array_element))
    (Utilities|Array|Add (Variables|Default|GetKDs) (Variables|/Game/Blueprints/MyPlayerController.MyPlayerController_C|GetKD _asmy_player_controller)))
  (while (> (Utilities|Array|Length (Variables|Default|GetKDs)) 0)
    (Utilities|Array|Add (Variables|Default|GetPlayerAddedToScoreBoard) (Utilities|Array|Get(acopy) (Variables|Default|GetCopies) _indexofmaxvalue))
    (Utilities|Array|RemoveIndex (Variables|Default|GetCopies) _indexofmaxvalue)
    (Utilities|Array|RemoveIndex (Variables|Default|GetKDs) _indexofmaxvalue))
  (for _array_element_2 (Variables|Default|GetAllPCs)
    (bind _asmy_player_controller_2 (Utilities|Casting|CastToMyPlayerController _array_element_2))
    (Default|SetServerData _asmy_player_controller_2 (Variables|Default|GetServerName) (Variables|Default|GetServerMode))
    (Default|ClearScoreBoard _asmy_player_controller_2)
    (for (_array_element_3 _array_index) (Variables|Default|GetPlayerAddedToScoreBoard)
      (bind _asmy_player_controller_3 (Utilities|Casting|CastToMyPlayerController _array_element_3))
      (if (< _array_index (Variables|Default|GetMaxPlayerInTopList))
        (if (== _array_element_2 _array_element_3)
          (Variables|Default|SetIsOwnPlayer? true)
          (else
            (Variables|Default|SetIsOwnPlayer? false)))
        (Default|AddPlayerScoreBoard _asmy_player_controller_2 (Class|AdvancedSessionsLibrary|GetPlayerName _array_element_3) (Variables|/Game/Blueprints/MyPlayerController.MyPlayerController_C|GetKills _asmy_player_controller_3) (Variables|/Game/Blueprints/MyPlayerController.MyPlayerController_C|GetDeath _asmy_player_controller_3) (+ _array_index 1) (Variables|/Game/Blueprints/MyPlayerController.MyPlayerController_C|GetKD _asmy_player_controller_3) (Variables|Default|GetIsOwnPlayer?) false)
        (elif (== _asmy_player_controller_3 _asmy_player_controller_2)
          (Default|AddPlayerScoreBoard _asmy_player_controller_2 (Class|AdvancedSessionsLibrary|GetPlayerName _array_element_3) (Variables|/Game/Blueprints/MyPlayerController.MyPlayerController_C|GetKills _asmy_player_controller_3) (Variables|/Game/Blueprints/MyPlayerController.MyPlayerController_C|GetDeath _asmy_player_controller_3) (+ _array_index 1) (Variables|/Game/Blueprints/MyPlayerController.MyPlayerController_C|GetKD _asmy_player_controller_3) true true))))))

(event Custom|TeleportOnEachPlayer
  (switch int (Variables|Default|GetGameMode)
    (:1
      (for (_array_element _array_index) (Variables|Default|GetAllPCs)
        (bind _returnvalue (Game|SpawnActorfromClass "/Game/ThirdPersonBP/Blueprints/Character1.Character1_C" (Math|Transform|MakeTransform (Transformation|GetWorldLocation (Variables|/Game/Blueprints/SpawnPoints/DefaultSpawnPoint.DefaultSpawnPoint_C|GetSphere (Utilities|Array|Get(acopy) (Variables|Default|GetDefault%20Spawn) _array_index)))) "Undefined" 0 0))
        (Pawn|Possess _array_element _returnvalue)))
    (:2
      (for (_array_element_2 _array_index_2) (Variables|Default|GetAllPCs)
        (bind _returnvalue_2 (Game|SpawnActorfromClass "/Game/ThirdPersonBP/Blueprints/Character1.Character1_C" (Math|Transform|MakeTransform (Transformation|GetWorldLocation (Variables|/Game/Blueprints/SpawnPoints/SpawnPoint_1vs1.SpawnPoint_1vs1_C|GetSphere (Utilities|Array|Get(acopy) (Variables|Default|Get1vs1Spawn) _array_index_2)))) "Undefined" 0 0))
        (Pawn|Possess _array_element_2 _returnvalue_2)))))

(event Custom|CreateGameUIOnEachPlayer
  (for _array_element (Variables|Default|GetAllPCs)
    (bind _asmy_player_controller (Utilities|Casting|CastToMyPlayerController _array_element))
    (Default|CreateGameUi _asmy_player_controller)
    (CallFunction|UpdateScoreBoard)
    (switch int (Variables|Default|GetGameMode)
      (:1
        (Default|StartCountdownCenter _asmy_player_controller 0 5 true))
      (:2
        (Default|StartCountdownCenter _asmy_player_controller 0 7 false)))))

(event Custom|ToggleInGame
  (params (Now%20InGame? :type Boolean))
  (bind _asmy_game_instance (Utilities|Casting|CastToMyGameInstance (Game|GetGameInstance)))
  (Default|ToggleinGame _asmy_game_instance Now%20InGame?))

(event EventOnLogout
  (params (ExitingController :type Controller%20Object%20Reference))
  (bind _allpcs (Variables|Default|GetAllPCs))
  ;[1 1 1] Remove Player Controller
  (bind (_array_element _array_index) (Utilities|Array|ForEachLoopwithBreak _allpcs :!label _label)
    (:LoopBody
      (if (== ExitingController _array_element)
        (CallFunction|SendServerMssage (Utilities|String|Append (Class|AdvancedSessionsLibrary|GetPlayerName _array_element) " : " "Left"))
        (goto _label Break)))
    (:Completed
      (Utilities|Array|RemoveIndex _allpcs _array_index)
      (CallFunction|UpdateServer))))

(event EventOnSwapPlayerControllers
  (params (OldPC :type Player%20Controller%20Object%20Reference) (NewPC :type Player%20Controller%20Object%20Reference))
  (if (not (Variables|Default|GetTestMode))
    (Utilities|Array|Add (Variables|Default|GetPCsNeedToSetUp) NewPC)
    (Utilities|Array|Add (Variables|Default|GetAllPCs) NewPC)
    (Utilities|FlowControl|Delay 1.0)
    (CallFunction|SetServerDataGameplay)
    (Utilities|FlowControl|Delay 1.0)
    (CallFunction|UpdateScoreBoard)))

(event EventPostLogin
  (params (NewPlayer :type Player%20Controller%20Object%20Reference))
  (if (Variables|Default|GetTestMode)
    (Utilities|Array|Add (Variables|Default|GetPCsNeedToSetUp) NewPlayer)
    (Utilities|Array|Add (Variables|Default|GetAllPCs) NewPlayer)
    (Utilities|FlowControl|Delay 1.0)
    (CallFunction|SetServerDataGameplay)
    (Utilities|FlowControl|Delay 1.0)
    (CallFunction|UpdateScoreBoard)
    (else
      (Networking|SwitchHasAuthority
        (:Authority
          ;[1 1 1] Add each Player Controller to list and add server information
          (if (== (Variables|Default|GetGameMode) 0)
            (Utilities|Array|Add (Variables|Default|GetAllPCs) NewPlayer)
            (Variables|Default|SetPlyersInGamePlay (Variables|Default|GetAllPCs))
            (else
              (Utilities|Array|Add (Variables|Default|GetAllPCs) NewPlayer)))
          (bind _asmy_game_instance (Utilities|Casting|CastToMyGameInstance (Game|GetGameInstance)))
          (Variables|Default|SetServerName (Variables|/Game/Blueprints/MyGameInstance.MyGameInstance_C|GetServerName _asmy_game_instance))
          (Variables|Default|SetServerMap (Variables|/Game/Blueprints/MyGameInstance.MyGameInstance_C|GetServerMap _asmy_game_instance))
          (Variables|Default|SetServerMode (Variables|/Game/Blueprints/MyGameInstance.MyGameInstance_C|GetServerMode _asmy_game_instance))
          (Variables|Default|SetServerSlots (Variables|/Game/Blueprints/MyGameInstance.MyGameInstance_C|GetServerSlots _asmy_game_instance))
          (bind _asmy_player_controller (Utilities|Casting|CastToMyPlayerController NewPlayer))
          (Default|PlayerDataSetup _asmy_player_controller))))))

(event EventBeginPlay
  (Utilities|FlowControl|Sequence
    (:then_1
      (bind _outactors (Actor|GetAllActorsOfClass "/Game/Blueprints/SpawnPoints/DefaultSpawnPoint.DefaultSpawnPoint_C"))
      (bind _output_get (Variables|Default|SetDefault%20Spawn _outactors))
      (Utilities|Array|Shuffle _output_get))
    (:then_2
      (bind _outactors_2 (Actor|GetAllActorsOfClass "/Game/Blueprints/SpawnPoints/SpawnPoint_1vs1.SpawnPoint_1vs1_C"))
      (bind _output_get_2 (Variables|Default|Set1vs1Spawn _outactors_2))
      (Utilities|Array|Shuffle _output_get_2))))

(fn ConstructionScript)

(fn OnRepPCsNeedtoSetUp)